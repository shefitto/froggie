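; SpawnerStalk is a spawner that builds a vertical beanstalk by spawning one segment actor per Tick.
; While CurrentCount is at or below MaxActorCount, each spawn becomes CurrentActor, increments the count and raises CurrentLocation by a fixed Z step.
; BeginPlay only sets CurrentActor to itself; the logic reading location and rotation from CurrentActor never runs, so stacking starts at CurrentLocation's default.
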(event EventBeginPlay
  (Variables|Default|SetCurrentActor self))

(event EventTick
  (params (DeltaSeconds :type Float%20%28single-precision%29))
  (if (<= (Variables|Default|GetCurrentCount) (Variables|Default|GetMaxActorCount))
    (bind _returnvalue (Game|SpawnActorfromClass "/Game/Blueprints/Beanstalk.Beanstalk_C" (Math|Transform|MakeTransform (Variables|Default|GetCurrentLocation) "0, 0, 0" "1.000000,1.000000,1.000000") "Undefined" "MultiplyWithRoot" 0 0))
    (Variables|Default|SetCurrentActor _returnvalue)
    (Variables|Default|SetCurrentCount (+ (Variables|Default|GetCurrentCount) 1))
    (Variables|Default|SetCurrentLocation (+ (Variables|Default|GetCurrentLocation) "0.000000,0.000000,200.000000"))))

(fn ConstructionScript)